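; Base character Blueprint with a zoomable third-person camera, a hold-to-free-look mode and player body-swapping between characters.
; The swap input box-traces from the camera, and a sufficiently distant target character briefly shows a trigger plate rotated toward the sender.
; A character overlapping that plate hands possession to its owner, with a helper camera moving from the previous view.
; A sphere-trace sense input adds non-character hits to the trace ignore list.
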(event OnComponentBeginOverlap(StaticMesh)
  (params (OverlappedComponent :type Primitive%20Component%20Object%20Reference) (OtherActor :type Actor%20Object%20Reference) (OtherComp :type Primitive%20Component%20Object%20Reference) (OtherBodyIndex :type Integer) (bFromSweep :type Boolean) (SweepResult :type Hit%20Result%20Structure%20%28by%20ref%29))
  (bind _returnvalue (Game|GetPlayerController 0))
  ;[1 1 1] Pawn Swap On Overlap
  (bind _asbp_char_base (Utilities|Casting|CastToBP_CharBase OtherActor))
  (if (Variables|Default|GetbCharacterSwapAvailable)
    (CallFunction|ToggleSwapTriggerPlate false)
    (Pawn|UnPossess _returnvalue)
    (|CameraRotation (Variables|BP_CharBase_C|GetCamera_3rd _asbp_char_base))
    (Pawn|Possess _returnvalue self)
    (CallFunction|SetBlockControllers true)
    (Components|MoveComponentTo (Variables|Default|GetCameraForPawnRotate) "-300.000000,0.000000,89.000000" "0, 0, 0" true true (Variables|Camera|GetCameraBlendDuration) false)
    (CallFunction|SwitchCameraViewonRotatePawn true)
    (CallFunction|SetBlockControllers false)))

(event EventPossessed
  (params (NewController :type Controller%20Object%20Reference))
  (|InitPlayerStateRef))

(event EventUnpossessed
  (params (OldController :type Controller%20Object%20Reference))
  ;[1 1 1] Actor free
  (CallFunction|ToggleSwapTriggerPlate false)
  (Transformation|SetRelativeRotation (Variables|Default|GetSpringArm_SwapTrigger) "0,180.000000, 0" false false)
  (Transformation|SetRelativeRotation (Variables|Components|GetSpringArm_3rd) "0, 0, 0" false false))

(event EventBeginPlay
  ;[1 1 1] Begin play Init
  (Utilities|FlowControl|Sequence
    (:then_0
      (CallFunction|ToggleSwapTriggerPlate false))
    (:then_2
      (|BindEventBeginSwapPawnTransformation))
    (:then_3
      (|InitCamera))
    (:then_4
      (Variables|PawnRotation|SetTraceLength 5e+03))
    (:then_5
      (Variables|/Script/Engine.CharacterMovementComponent|SetGravityScale (Variables|Character|GetCharacterMovement) 1.0))))

(event Input|ActionEvents|InputActionCameraFree
  (params (Key :type Key%20Structure :default "None"))
  (bind _springarm_3rd (Variables|Components|GetSpringArm_3rd))
  ;[1 1 1] Free camera
  (:Pressed
    (bind _output_get (Variables|Camera|SetbCameraConnected false))
    (Variables|/Script/Engine.SpringArmComponent|SetbUsePawnControlRotation _springarm_3rd _output_get))
  (:Released
    (Camera|AddControllerNoclipInput (Variables|Camera|GetCameraYawDelta) (Variables|Camera|GetCameraPitchDelta))
    (bind _output_get_2 (Variables|Camera|SetbCameraConnected true))
    (Variables|/Script/Engine.SpringArmComponent|SetbUsePawnControlRotation _springarm_3rd _output_get_2)))

(event Input|ActionEvents|InputActionEscapeKey
  (params (Key :type Key%20Structure :default "None"))
  (:Released
    (Game|QuitGame 0 "Quit" false)))

(event Input|AxisEvents|InputAxisSwapCharacters
  (params (AxisValue :type Float%20%28single-precision%29))
  ;[1 1 1] Beam/Ray Sender
  (Utilities|AxisFilterZeros AxisValue)
  (bind (_startray _endray _actorstoignore) (CallFunction|MakeTraceDirection))
  (bind _outhit (Collision|BoxTraceByChannel _startray _endray "50.000000,50.000000,50.000000" "0, 0, 0" "TraceTypeQuery2" false _actorstoignore "ForOneFrame"))
  (if (.bBlockingHit (Collision|BreakHitResult _outhit))
    (bind _asbp_char_base (Utilities|Casting|CastToBP_CharBase (.HitActor (Collision|BreakHitResult _outhit))))
    (if (.bDistanceMoreThenArm (|DistansFromSelfToTarget _asbp_char_base))
      (Variables|BP_CharBase_C|SetPawnTransformSender (.Target-Out (|DistansFromSelfToTarget _asbp_char_base)) self)
      (Default|CallBeginSwapPawnTransformation (.Target-Out (|DistansFromSelfToTarget _asbp_char_base))))))

(event Input|AxisEvents|InputAxisSenseCharacters
  (params (AxisValue :type Float%20%28single-precision%29))
  ;[1 1 1] Sphere scan
  (Utilities|AxisFilterZeros AxisValue)
  (bind (_startray _endray _actorstoignore) (CallFunction|MakeTraceDirection))
  (bind _outhits (Collision|MultiSphereTraceByChannel _startray _endray 1e+03 "TraceTypeQuery2" true _actorstoignore "None"))
  (bind _array_element (Utilities|Array|ForEachLoopwithBreak _outhits)
    (:LoopBody
      (if true
        (Utilities|Casting|CastToBP_CharBase (.HitActor (Collision|BreakHitResult _array_element))
          (:CastFailed
            (Utilities|Array|AddUnique (Variables|PawnRotation|GetActorsToIgnore) (.HitActor (Collision|BreakHitResult _array_element)))))))))

(event Input|AxisEvents|InputAxisCameraDistance
  (params (AxisValue :type Float%20%28single-precision%29))
  (bind _springarm_3rd (Variables|Components|GetSpringArm_3rd))
  ;[1 1 1] Camera Distance
  (bind _val_out (Utilities|AxisFilterZeros AxisValue))
  (Utilities|IsCameraNotBlock)
  (Variables|/Script/Engine.SpringArmComponent|SetTargetArmLength _springarm_3rd (+ (* _val_out 5.0) (Variables|/Script/Engine.SpringArmComponent|GetTargetArmLength _springarm_3rd))))

(event Input|AxisEvents|InputAxisCameraTurn
  (params (AxisValue :type Float%20%28single-precision%29))
  ;[1 1 1] Camera View
  (Utilities|IsCameraNotBlock)
  (bind (_yaw_out _pitch_out) (|Marshroot_Input AxisValue (stale Input|AxisEvents|InputAxisCameraLookUp AxisValue))
    (:Yaw%20Exec
      (Pawn|Input|AddControllerYawInput _yaw_out))
    (:Pitch%20Exec
      (Pawn|Input|AddControllerPitchInput _pitch_out))
    (:Noclip
      (Camera|AddControllerNoclipInput _yaw_out _pitch_out))))

(event Input|AxisEvents|InputAxisCameraLookUp
  (params (AxisValue :type Float%20%28single-precision%29))
  ;[1 1 1] Camera View
  (Utilities|IsCameraNotBlock)
  (|Marshroot_Input (stale Input|AxisEvents|InputAxisCameraTurn AxisValue) AxisValue) ; enters at Pitch - LookUp
)

(fn ConstructionScript)

(fn AddControllerNoclipInput
  (params (Yaw :type Float%20%28single-precision%29) (Pitch :type Float%20%28single-precision%29))
  (Transformation|AddRelativeRotation (Variables|Components|GetSpringArm_3rd) (Math|Rotator|MakeRotator 0.0 Pitch Yaw) false false)
  (Variables|Camera|SetCameraYawDelta (- (Variables|Camera|GetCameraYawDelta) Yaw))
  (Variables|Camera|SetCameraPitchDelta (- (Variables|Camera|GetCameraPitchDelta) Pitch)))

(fn MakeTraceDirection
  (bind _camera_3rd (Variables|Components|GetCamera_3rd))
  (bind _returnvalue (Transformation|GetWorldLocation _camera_3rd))
  (return _returnvalue (+ _returnvalue (* (Math|Vector|GetForwardVector _camera_3rd) (Variables|PawnRotation|GetTraceLength))) (Variables|PawnRotation|GetActorsToIgnore)))

(fn ToggleSwapTriggerPlate
  (params (Visible :type Boolean))
  (bind _staticmesh (Variables|Default|GetStaticMesh))
  (bind _output_get (Variables|Default|SetbCharacterSwapAvailable Visible))
  (bind _output_get_2 (Variables|/Script/Engine.PrimitiveComponent|SetbGenerateOverlapEvents _staticmesh _output_get))
  (Development|SetHiddeninGame _staticmesh (not _output_get_2) true))

(fn HideSwapTriggerPlate
  (CallFunction|ToggleSwapTriggerPlate false))

(fn SwitchCameraViewonRotatePawn
  (params (ToDefault :type Boolean))
  (Components|Activation|SetActive (Variables|Default|GetCameraForPawnRotate) (not ToDefault) false)
  (Components|Activation|SetActive (Variables|Components|GetCamera_3rd) ToDefault false))

(fn SetBlockControllers
  (params (bBlock :type Boolean))
  (bind _returnvalue (Game|GetPlayerController 0))
  (Input|SetIgnoreMoveInput _returnvalue bBlock)
  (Input|SetIgnoreLookInput _returnvalue bBlock))

(event Custom|BeginSwapPawnTransformation_Event
  (bind (_beforenormalizelength _returnvector) (|GetNormalDirection))
  (bind _springarm_swaptrigger (Variables|Default|GetSpringArm_SwapTrigger))
  ;[1 1 1] Rotate trigger plane to current actor
  (CallFunction|ToggleSwapTriggerPlate true)
  (Utilities|Time|SetTimerbyFunctionName 0 "HideSwapTriggerPlate" 5.0)
  (Timeline|Timeline_0 PlayFromStart
    (:Update
      (if (not (>= _beforenormalizelength (Variables|/Script/Engine.SpringArmComponent|GetTargetArmLength _springarm_swaptrigger)))
        (Timeline|Timeline_0 Stop)
        (else
          (Transformation|SetWorldRotation _springarm_swaptrigger (Math|Conversions|RotationFromXVector _returnvector) true false))))))