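; Robot player character with camera-relative movement, a stamina-limited strafe dash and a toe-thruster follow-up jump.
; Strafe sweeps the capsule along a timeline in the input direction, or backward without input, blocking controls and starting a cooldown; re-pressing cancels it.
; Holding a follow-up jump extends hold time, shows toe fire and drains stamina on Tick until release or exhaustion.
; Stamina lives in a widget referenced through the PlayerState.
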(event EventPossessed
  (params (NewController :type Controller%20Object%20Reference))
  (|CallParentFunction 0)
  (CallFunction|FireVisibility false))

(event EventBeginPlay
  (|CallParentFunction)
  (CallFunction|FireVisibility false))

(fn ConstructionScript
  (CallFunction|FireVisibility false))

(fn ScaleMoveWhileJump
  (params (Axis :type Float%20%28single-precision%29))
  (return (Math|Float|Lerp (* 100 Axis) Axis (Math|Conversions|ToFloat(Boolean) (Variables|Default|GetbPressedJump)))))

(fn EnableStraif
  (Variables|Straif|SetbStraifAvailable true))

(fn FireVisibility
  (params (bVisible :type Boolean))
  (Rendering|SetVisibility (Variables|Default|GetR_Toe_Fire) bVisible true)
  (Rendering|SetVisibility (Variables|Default|GetL_Toe_Fire) bVisible true))

(fn StopJump
  (Variables|Default|SetJumpMaxHoldTime (Variables|Jump|GetJump%20Default%20Hold%20Time))
  (Character|StopJumping)
  (CallFunction|FireVisibility false))

(fn FnConsumeStamina
  (params (BP%20PlayerState :type BP%20Player%20State%20Object%20Reference) (Consume :type Float%20%28single-precision%29))
  (bind _ref_wb_stamina (Variables|/Game/Blueprint/BP_PlayerState.BP_PlayerState_C|GetRef_WB_Stamina BP%20PlayerState))
  (Default|ConsumeStaminaInst _ref_wb_stamina Consume)
  (return (Variables|/Game/Blueprint/Interface/WB_Stamina.WB_Stamina_C|GetbOutOfStamina _ref_wb_stamina)))

(fn IsStaminaNotEmpty
  (return (not (Variables|/Game/Blueprint/Interface/WB_Stamina.WB_Stamina_C|GetbOutOfStamina (Variables|/Game/Blueprint/BP_PlayerState.BP_PlayerState_C|GetRef_WB_Stamina (Variables|Default|GetRef_BP_PlayerState))))))

(event Input|ActionEvents|InputActionMoveStraif
  (params (Key :type Key%20Structure :default "None"))
  (bind (_forward _right) (|GetNormalizeDirections))
  (bind _straif_length (Variables|Straif|GetStraif%20Length))
  (bind _moveprecission (Variables|Default|GetMovePrecission))
  ;[1 1 1] Shift (Straif to dir)
  (:Pressed
    (Utilities|IsStraifAvailable
      (:then
        (bind _returnvalue (CallFunction|IsStaminaNotEmpty))
        (if _returnvalue
          (Variables|Straif|SetbStraifAvailable false)
          (Utilities|Time|SetTimerbyFunctionName 0 "enableStraif" 1.0)
          (Variables|Straif|SetStraif%20Direction (Math|Vector|Lerp(Vector) (* (Math|Vector|Normalize (+ (* _forward (stale Input|AxisEvents|InputAxisMoveForward _val_out)) (* _right (stale Input|AxisEvents|InputAxisMoveRight _val_out))) _moveprecission) _straif_length) (* _forward (* _straif_length -1.0)) (Math|Conversions|ToFloat(Boolean) (Math|Vector|Equal(Vector) (+ (* _forward (stale Input|AxisEvents|InputAxisMoveForward _val_out)) (* _right (stale Input|AxisEvents|InputAxisMoveRight _val_out))) "0, 0, 0" _moveprecission))))
          (CallFunction|SetBlockControllers true)
          (|StraifProcess :!label _label
            (:Finished
              (CallFunction|SetBlockControllers false :!label _label_2)))))
      (:StraifOnGoing
        (Utilities|FlowControl|Sequence
          (:then_0
            (goto _label Stop))
          (:then_1
            (goto _label_2)))))))

(event Input|AxisEvents|InputAxisMoveForward
  (params (AxisValue :type Float%20%28single-precision%29))
  ;[1 1 1] WASD
  (bind _val_out (Utilities|AxisFilterZeros AxisValue))
  (Utilities|IsInputEnable
    (:then
      (Pawn|Input|AddMovementInput (.Forward (|GetNormalizeDirections)) _val_out false))))

(event Input|AxisEvents|InputAxisMoveRight
  (params (AxisValue :type Float%20%28single-precision%29))
  ;[1 1 1] WASD
  (bind _val_out (Utilities|AxisFilterZeros AxisValue))
  (Utilities|IsInputEnable
    (:then
      (Pawn|Input|AddMovementInput (.Right (|GetNormalizeDirections)) _val_out true))))

(event EventTick
  (params (DeltaSeconds :type Float%20%28single-precision%29))
  ;[1 1 1] Jump Stamina Drain
  (if (Variables|Default|GetbPressedJump)
    (if (not (Utilities|IsFirstJump))
      (bind _out_of_stamina (CallFunction|FnConsumeStamina (Variables|Default|GetRef_BP_PlayerState) (Variables|Default|GetStaminaJumpConsumeOvertime)))
      (if _out_of_stamina
        (CallFunction|StopJump)))))

(event Input|ActionEvents|InputActionMoveJump
  (params (Key :type Key%20Structure))
  (bind _bfirstjump (Utilities|IsFirstJump))
  ;[1 1 1] Jump Control
  (:Pressed
    (Utilities|IsInputEnable
      (:then
        (bind _returnvalue (CallFunction|IsStaminaNotEmpty))
        (if _returnvalue
          (if _bfirstjump
            _
            (else
              (Variables|Default|SetJumpMaxHoldTime (Variables|Jump|GetJump%20Maximum%20Hold%20Time))))
          (|JumpNode _bfirstjump)))))
  (:Released
    (CallFunction|StopJump)))