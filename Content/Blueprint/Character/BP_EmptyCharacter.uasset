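; BP_EmptyCharacter is a cursor-driven placeholder character from which the player picks another pawn to control.
; It shows the mouse cursor on BeginPlay, and a left click traces for Pawn objects under it, prints the hit name, then possesses that pawn and hides the cursor.
; Holding the right mouse button lets mouse movement nudge the default camera's pitch and yaw, each clamped to a small symmetric range.
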(event EventBeginPlay
  (Variables|/Script/Engine.PlayerController|SetbShowMouseCursor (Game|GetPlayerController 0) true))

(event Input|MouseEvents|RightMouseButton
  (params (Key :type Key%20Structure))
  (:Pressed
    (Variables|Default|SetbCameraMove true))
  (:Released
    (Variables|Default|SetbCameraMove false)))

(event Input|MouseEvents|LeftMouseButton
  (params (Key :type Key%20Structure))
  (bind _returnvalue (Game|GetPlayerController 0))
  (bind _array (Utilities|Array|MakeArray "ObjectTypeQuery3"))
  (bind _hitresult (Class|PlayerController|GetHitResultUnderCursorforObjects _returnvalue _array true))
  (bind _hitactor (Collision|BreakHitResult _hitresult))
  (:Pressed
    (Development|PrintString (Utilities|GetDisplayName _hitactor))
    (bind _aspawn (Utilities|Casting|CastToPawn _hitactor))
    (Pawn|UnPossess _returnvalue)
    (Pawn|Possess _returnvalue _aspawn)
    (Variables|/Script/Engine.PlayerController|SetbShowMouseCursor (Game|GetPlayerController 0) false)))

(event Input|MouseEvents|Mouse2D
  (params (AxisValue :type Vector :default "0, 0, 0"))
  (|LittleMoveCamera (.x AxisValue) (.y AxisValue)))

(fn ConstructionScript)

(fn GetLimitedAngle
  (params (Angle :type Float%20%28single-precision%29) (CurrentAngle :type Float%20%28single-precision%29))
  (bind _returnvalue (* Angle 0.1))
  (bind _returnvalue_2 (+ _returnvalue CurrentAngle))
  (return (* (Math|Float|Sign(Float) _returnvalue_2) (Math|Float|Min(Float) (Math|Float|Absolute(Float) _returnvalue_2) (Math|Float|MakeLiteralFloat 3e+01)))))