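; A free-flying "NoClip" character that turns off gravity on BeginPlay and moves along its local forward, right and up axes.
; MoveForward, MoveRight and JumpRate inputs pass a zero filter, then become fixed-step offsets scaled by axis value and frame time relative to the game mode's default.
; FnInput also respects ignored move input.
; AddActorLocalOffset applies each offset directly with sweep on, so blocking collision can still stop it.
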(event EventBeginPlay
  ;[1 1 1] Begin Play
  (|CallParentFunction)
  (Variables|/Script/Engine.CharacterMovementComponent|SetGravityScale (Variables|Character|GetCharacterMovement) 0.0))

(event Input|AxisEvents|InputAxisJumpRate
  (params (AxisValue :type Float%20%28single-precision%29))
  ;[1 1 1] Up/Down
  (bind _val_out (Utilities|AxisFilterZeros AxisValue))
  (bind _deltalocation (Utilities|FnInput "0,0,10.000000" _val_out))
  (Transformation|AddActorLocalOffset _deltalocation true false))

(event Input|AxisEvents|InputAxisMoveForward
  (params (AxisValue :type Float%20%28single-precision%29))
  ;[1 1 1] WASD
  (bind _val_out (Utilities|AxisFilterZeros AxisValue))
  (bind _deltalocation (Utilities|FnInput "10.000000,0,0" _val_out))
  (Transformation|AddActorLocalOffset _deltalocation true false))

(event Input|AxisEvents|InputAxisMoveRight
  (params (AxisValue :type Float%20%28single-precision%29))
  ;[1 1 1] WASD
  (bind _val_out (Utilities|AxisFilterZeros AxisValue))
  (bind _deltalocation (Utilities|FnInput "0,10.000000,0" _val_out))
  (Transformation|AddActorLocalOffset _deltalocation true false))

(fn ConstructionScript)