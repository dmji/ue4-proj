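; BP_PlayerState is a player state Blueprint that holds setup logic for the stamina and aim HUD overlays.
; InitStamina stores a WB_Stamina widget reference, makes it fully opaque and adds it to the viewport, while InitAim creates and displays a WB_Aim widget.
; The chain that creates the stamina widget and calls both functions is disconnected from the empty BeginPlay, so this graph never shows either overlay.
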(event EventBeginPlay
  ;[1 1 1] Overlay Init
)

(fn ConstructionScript)